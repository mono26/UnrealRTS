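; Actor component for the RTS that gives its owner interaction points and a radius for interactors.
; GetClosestInteractionPointTo searches the owner's BP_InteractionPointComponents by squared distance and returns the one nearest the interactor, drawing a debug sphere there.
; It returns nothing when the interactor is invalid, which also prints a message, or when the owner has no points.
; GetInteractableRadius scales the base radius by the owner's X scale.
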(fn `GetClosestInteractionPointTo`
  (params (InteractorRef :type "Actor Object Reference"))
  (returns (InteractionPoint :type "SceneComponent Object Reference"))
  (locals (ClosestSqrDistance :type "Float (double-precision)") (ClosestPoint :type "SceneComponent Object Reference"))
  (bind _returnvalue (`Actor.K2_GetComponentsByClass` (`self.GetOwner`) "/Game/MyFirstRTS/Core/Building/BP_InteractionPointComponent.BP_InteractionPointComponent_C"))
  (`/Engine/EditorBlueprintResources/StandardMacros.IsValid` InteractorRef
    (:`Is Valid`
      (if (`KismetArrayLibrary.Array_IsNotEmpty` _returnvalue)
        (set `local.ClosestSqrDistance` 1e+17)
        (set `local.ClosestPoint` null)
        (for _array_element _returnvalue
          (bind _returnvalue_2 (`KismetMathLibrary.Vector_DistanceSquared` (`Actor.K2_GetActorLocation` InteractorRef) (`SceneComponent.K2_GetComponentLocation` _array_element)))
          (if (< _returnvalue_2 (`local.ClosestSqrDistance`))
            (set `local.ClosestSqrDistance` _returnvalue_2)
            (set `local.ClosestPoint` _array_element)))
        (`KismetSystemLibrary.DrawDebugSphere` (`SceneComponent.K2_GetComponentLocation` (`local.ClosestPoint`)) 100.0 12 (struct :`R` 1.0 :`B` 0.864954 :`A` 1.0) 3.0 1.0)
        (return (`local.ClosestPoint`))
        (else
          _)))
    (:`Is Not Valid`
      (`KismetSystemLibrary.PrintString` "Not a valid interactor ref.")))
  (return null))

(fn `GetInteractableRadius`
  (returns (Radius :type "Float (double-precision)"))
  (bind _returnvalue_x (`KismetMathLibrary.BreakVector` (`Actor.GetActorScale3D` (`self.GetOwner`))))
  (return (* (`self.InteractableRadius`) _returnvalue_x)))