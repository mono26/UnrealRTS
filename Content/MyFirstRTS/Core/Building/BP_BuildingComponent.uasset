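; BP_BuildingComponent is an RTS building component that gives its owning actor health, selection and interaction behavior.
; On BeginPlay it adds and configures health bar, selection and interactable components, sizing the latter two from the building's size.
; Selection and click events are forwarded to PC_MyFirstRTS, with selectability limited to Friendly buildings.
; Damage bound from the owner lowers clamped health, refreshes the bar and fires OnHealthZero at zero.
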(event `self.ReceiveBeginPlay`
  (bind _returnvalue (`self.GetOwner`))
  (`|ExecutionSequence`
    (:`then_0`
      (set `self.HealthCurrent` (`self.HealthMax`))
      (bind _returnvalue_2 (`|AddComponentByClass` _returnvalue "/Game/MyFirstRTS/Core/Unit/BP_HealthBarComponent.BP_HealthBarComponent_C" false (`KismetMathLibrary.MakeTransform` (`self.HealthBarLocalPos`))))
      (bind _output_get (set `self.HealthBarComponent` _returnvalue_2))
      (`WidgetComponent.SetDrawSize` _output_get (`self.HealthBarSize`))
      (`self.UpdateHealthBar`))
    (:`then_1`
      (bind _returnvalue_3 (`|AddComponentByClass` _returnvalue "/Game/MyFirstRTS/Core/Building/BP_SelectionComponent.BP_SelectionComponent_C"))
      (bind _output_get_2 (set `self.SelectionComponentRef` _returnvalue_3))
      (set `/Game/MyFirstRTS/Core/Building/BP_SelectionComponent.IndicatorRadius` (`self.BuildingSize`) _output_get_2)
      (set `/Game/MyFirstRTS/Core/Building/BP_SelectionComponent.IndicatorCenter` (`self.BuildingCenter`) _output_get_2)
      (`/Game/MyFirstRTS/Core/Building/BP_SelectionComponent.UpdateDecal` _output_get_2))
    (:`then_2`
      (bind _returnvalue_4 (`|AddComponentByClass` _returnvalue "/Game/MyFirstRTS/Core/Building/BP_InteractableComponent.BP_InteractableComponent_C"))
      (bind _output_get_3 (set `self.InteractableComponent` _returnvalue_4))
      (set `/Game/MyFirstRTS/Core/Building/BP_InteractableComponent.InteractableRadius` (`self.BuildingSize`) _output_get_3))
    (:`then_3`
      (add `Actor.OnTakeAnyDamage` _returnvalue (`|CreateDelegate` :!event `OnDamage`)))))

(event `/Game/MyFirstRTS/Core/Building/BPI_ISelectable.OnSelected`
  (`|ExecutionSequence`
    (:`then_0`
      (bind _aspc_my_first_rts (cast `/Game/MyFirstRTS/Core/Player/PC_MyFirstRTS` (`GameplayStatics.GetPlayerController` 0)))
      (`/Game/MyFirstRTS/Core/Player/PC_MyFirstRTS.OnActorSelected` _aspc_my_first_rts (`self.GetOwner`)))
    (:`then_1`
      (`/Game/MyFirstRTS/Core/Building/BP_SelectionComponent.OnSelected` (`self.SelectionComponentRef`)))))

(event `/Game/MyFirstRTS/Core/Building/BPI_ISelectable.OnDeselected`
  (`|ExecutionSequence`
    (:`then_0`
      (bind _aspc_my_first_rts (cast `/Game/MyFirstRTS/Core/Player/PC_MyFirstRTS` (`GameplayStatics.GetPlayerController` 0)))
      (`/Game/MyFirstRTS/Core/Player/PC_MyFirstRTS.OnActorDeselected` _aspc_my_first_rts (`self.GetOwner`)))
    (:`then_1`
      (`/Game/MyFirstRTS/Core/Building/BP_SelectionComponent.OnDeselected` (`self.SelectionComponentRef`)))))

(event `/Game/MyFirstRTS/Core/Building/BPI_IClickable.OnCursorClicked`
  (bind _aspc_my_first_rts (cast `/Game/MyFirstRTS/Core/Player/PC_MyFirstRTS` (`GameplayStatics.GetPlayerController` 0)))
  (`/Game/MyFirstRTS/Core/Player/PC_MyFirstRTS.OnGameActorClicked` _aspc_my_first_rts (`self.GetOwner`)))

(event `OnDamage`
  (params (DamagedActor :type "Actor Object Reference") (Damage :type "Float (single-precision)") (DamageType :type "DamageType Object Reference") (InstigatedBy :type "Controller Object Reference") (DamageCauser :type "Actor Object Reference"))
  (bind _output_get (set `self.HealthCurrent` (`KismetMathLibrary.FMax` (- (`self.HealthCurrent`) Damage))))
  (`self.UpdateHealthBar`)
  (if (<= _output_get 0.0)
    (`self.OnHealthZero` (`self.GetOwner`))))

(fn `CanBeSelected`
  (returns (CanBeSelected :type Boolean))
  (return (`|EnumEquality` (`self.TeamAttitude`) "Friendly")))

(fn `UpdateHealthBar`
  (bind _returnvalue (`Actor.GetComponentByClass` (`self.GetOwner`) "/Game/MyFirstRTS/Core/Unit/BP_HealthBarComponent.BP_HealthBarComponent_C"))
  (`/Engine/EditorBlueprintResources/StandardMacros.IsValid` _returnvalue
    (:`Is Valid`
      (`/Game/MyFirstRTS/Core/Unit/BP_HealthBarComponent.UpdateHealthBar` _returnvalue (/ (`self.HealthCurrent`) (`self.HealthMax`))))))