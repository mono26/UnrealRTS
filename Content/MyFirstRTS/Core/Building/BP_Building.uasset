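; BP_Building is an RTS building actor that can be clicked, selected and destroyed.
; Click, selection, deselection and the can-be-selected query all forward to BPBuildingComponent, which holds that logic.
; When BP_HealthComponent reports zero health, it turns off the scene root's visibility without propagating to children, then destroys the actor after a short delay.
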(event `self.ReceiveActorOnClicked`
  (params (ButtonPressed :type "Key Structure"))
  (`self.OnCursorClicked`))

(event `self.OnCursorClicked`
  (`/Game/MyFirstRTS/Core/Building/BP_BuildingComponent.OnCursorClicked` (`self.BP_BuildingComponent`)))

(event `/Game/MyFirstRTS/Core/Component/BPI_ISelectable.OnSelected`
  (`/Game/MyFirstRTS/Core/Building/BP_BuildingComponent.OnSelected` (`self.BP_BuildingComponent`)))

(event `/Game/MyFirstRTS/Core/Component/BPI_ISelectable.OnDeselected`
  (`/Game/MyFirstRTS/Core/Building/BP_BuildingComponent.OnDeselected` (`self.BP_BuildingComponent`)))

(event `self.BP_HealthComponent.OnHealthZero`
  (bind _defaultsceneroot (`self.DefaultSceneRoot`))
  (`SceneComponent.SetVisibility` _defaultsceneroot false false)
  (`SceneComponent.SetHiddenInGame` _defaultsceneroot false false)
  (`KismetSystemLibrary.Delay` 0.5)
  (`self.K2_DestroyActor`))

(fn `CanBeSelected`
  (returns (CanBeSelected :type Boolean))
  (bind _canbeselected (`/Game/MyFirstRTS/Core/Building/BP_BuildingComponent.CanBeSelected` (`self.BP_BuildingComponent`)))
  (return _canbeselected))

(fn `UserConstructionScript`)