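; BP_ResourceComponent is an RTS component that makes its owner a gatherable resource with a limited number of gathers.
; GetGatheredResource decrements MineCount, fires OnResourceGathered, fires OnResourceExhausted once CanGather fails, and returns the resource type and amount per gather.
; CanGather only tests whether MineCount is above zero; GetGatheredResource does not check it before decrementing.
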(fn `CanGather`
  (returns (CanGather :type Boolean))
  (return (> (`self.MineCount`) 0)))

(fn `GetGatheredResource`
  (returns (ResourceType :type "/Game/MyFirstRTS/Core/Resource/E_ResourceType Enum") (GatherAmount :type Integer))
  (set `self.MineCount` (- (`self.MineCount`) 1))
  (`self.OnResourceGathered`)
  (`|ExecutionSequence`
    (:`then_0`
      (if (not (`self.CanGather`))
        (`self.OnResourceExhausted`)))
    (:`then_1`
      (return (`self.ResourceType`) (`self.AmountToGive`)))))