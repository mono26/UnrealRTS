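; BP_GatherIndicator is a short-lived actor that shows a mesh rising upward, likely as feedback for resource gathering.
; The construction script applies MeshToUse to its static mesh component.
; On BeginPlay a sped-up timeline drives the mesh's relative Z location up to MaxUpwardDistance, then the actor destroys itself when the timeline finishes.
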(event `self.ReceiveBeginPlay`
  (`TimelineComponent.SetPlayRate` (`self.UpwardsAnimation`) 3.0)
  (bind (_direction _zvaluemultiplier) (`Timeline|UpwardsAnimation`)
    (:`Update`
      (`SceneComponent.K2_SetRelativeLocation` (`self.StaticMesh`) (`KismetMathLibrary.MakeVector` 0.0 0.0 (* _zvaluemultiplier (`self.MaxUpwardDistance`))) false false))
    (:`Finished`
      (`self.K2_DestroyActor`))))

(fn `UserConstructionScript`
  (`StaticMeshComponent.SetStaticMesh` (`self.StaticMesh`) (`self.MeshToUse`)))