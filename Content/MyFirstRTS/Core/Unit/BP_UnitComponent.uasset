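; BP_UnitComponent gives its owning actor RTS unit behavior: health, a health bar and player selection.
; On BeginPlay it adds a health bar tinted by TeamComponent attitude and a selection decal sized to the unit, then binds to the owner's damage event.
; Damage lowers health, updates the bar and fires OnHealthZero at zero.
; Selection changes reach the decal and BP_PlayerCommander, while cursor clicks are forwarded only for friendly units.
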(event `self.ReceiveBeginPlay`
  (bind _returnvalue (`self.GetOwner`))
  (`|ExecutionSequence`
    (:`then_0`
      (bind _returnvalue_2 (`|AddComponentByClass` _returnvalue "/Game/MyFirstRTS/Core/Unit/BP_HealthBarComponent.BP_HealthBarComponent_C" false (`KismetMathLibrary.MakeTransform` (`self.HealthBarLocalPos`))))
      (bind _output_get (set `self.HealthbarComponent` _returnvalue_2))
      (`WidgetComponent.SetDrawSize` _output_get (`self.HealthBarSize`))
      (`/Game/MyFirstRTS/Core/Unit/BP_HealthBarComponent.UpdateHealthBarColor` _output_get (select `ETeamAttitude` (`TeamComponent.TeamAttitude` (`Actor.GetComponentByClass` (`self.GetOwner`) "/Script/MyFirstRTS.TeamComponent")) :`Friendly` (struct :`G` 1.0 :`A` 1.0) :`Neutral` (struct :`R` 1.0 :`G` 1.0 :`A` 1.0) :`Hostile` (struct :`R` 1.0 :`A` 1.0) :!type "LinearColor Structure"))
      (`self.UpdateHealthBar`))
    (:`then_1`
      (bind _returnvalue_3 (`|AddComponentByClass` _returnvalue "/Game/MyFirstRTS/Core/Building/BP_SelectionComponent.BP_SelectionComponent_C"))
      (bind _output_get_2 (set `self.SelectionComponentRef` _returnvalue_3))
      (set `/Game/MyFirstRTS/Core/Building/BP_SelectionComponent.IndicatorRadius` (`self.UnitSize`) _output_get_2)
      (set `/Game/MyFirstRTS/Core/Building/BP_SelectionComponent.IndicatorCenter` (`self.UnitCenter`) _output_get_2)
      (`/Game/MyFirstRTS/Core/Building/BP_SelectionComponent.UpdateDecal` _output_get_2))
    (:`then_4`
      (add `Actor.OnTakeAnyDamage` _returnvalue (`|CreateDelegate` :!event `OnDamage`)))))

(event `self.OnSelected`
  (`|ExecutionSequence`
    (:`then_0`
      (bind _asbp_player_commander (cast `/Game/MyFirstRTS/Core/Player/BP_PlayerCommander` (`GameplayStatics.GetPlayerController` 0)))
      (`/Game/MyFirstRTS/Core/Player/BP_PlayerCommander.OnActorSelected` _asbp_player_commander (`self.GetOwner`)))
    (:`then_1`
      (`/Game/MyFirstRTS/Core/Building/BP_SelectionComponent.OnSelected` (`self.SelectionComponentRef`)))))

(event `self.OnDeselected`
  (`|ExecutionSequence`
    (:`then_0`
      (bind _asbp_player_commander (cast `/Game/MyFirstRTS/Core/Player/BP_PlayerCommander` (`GameplayStatics.GetPlayerController` 0)))
      (`/Game/MyFirstRTS/Core/Player/BP_PlayerCommander.OnActorDeselected` _asbp_player_commander (`self.GetOwner`)))
    (:`then_1`
      (`/Game/MyFirstRTS/Core/Building/BP_SelectionComponent.OnDeselected` (`self.SelectionComponentRef`)))))

(event `/Game/MyFirstRTS/Core/Building/BPI_IClickable.OnCursorClicked`
  (bind _canbeselected (`self.CanBeSelected`))
  (if _canbeselected
    (bind _asbp_player_commander (cast `/Game/MyFirstRTS/Core/Player/BP_PlayerCommander` (`GameplayStatics.GetPlayerController` 0)))
    (`/Game/MyFirstRTS/Core/Player/BP_PlayerCommander.OnGameActorClicked` _asbp_player_commander (`self.GetOwner`))))

(event `OnDamage`
  (params (DamagedActor :type "Actor Object Reference") (Damage :type "Float (single-precision)") (DamageType :type "DamageType Object Reference") (InstigatedBy :type "Controller Object Reference") (DamageCauser :type "Actor Object Reference"))
  (bind _output_get (set `self.HealthCurrent` (`KismetMathLibrary.FMax` (- (`self.HealthCurrent`) Damage))))
  (`self.UpdateHealthBar`)
  (if (<= _output_get 0.0)
    (`self.OnHealthZero` (`self.GetOwner`))))

(fn `CanBeSelected`
  (returns (CanBeSelected :type Boolean))
  (return (`|EnumEquality` (`TeamComponent.TeamAttitude` (`Actor.GetComponentByClass` (`self.GetOwner`) "/Script/MyFirstRTS.TeamComponent")) "Friendly")))

(fn `OnActorClicked`
  (params (TouchedActor :type "Actor Object Reference") (ButtonPressed :type "Key Structure" :default "None"))
  (if (== TouchedActor (`self.GetOwner`))
    (`self.OnSelected`)))

(fn `UpdateHealthBar`
  (bind _healthbarcomponent (`self.HealthbarComponent`))
  (`/Engine/EditorBlueprintResources/StandardMacros.IsValid` _healthbarcomponent
    (:`Is Valid`
      (`/Game/MyFirstRTS/Core/Unit/BP_HealthBarComponent.UpdateHealthBar` _healthbarcomponent (/ (`self.HealthCurrent`) (`self.HealthMax`))))))