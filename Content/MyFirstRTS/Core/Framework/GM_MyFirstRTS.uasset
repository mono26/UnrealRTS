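; Game mode for the RTS that tracks townhalls and triggers the lose condition.
; On BeginPlay it gathers all BP_Townhall actors and binds to each building component's health-zero event.
; Destroyed townhalls leave the list, and a Friendly one brings up the lose screen widget.
; GetPlayerTownhall searches for a "Player" tag but indexes the townhall list by that tag's position, not the townhall's.
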(event `self.ReceiveBeginPlay`
  (bind _outactors (`GameplayStatics.GetAllActorsOfClass` "/Game/MyFirstRTS/Buildings/Townhall/BP_Townhall.BP_Townhall_C"))
  (bind _output_get (set `self.Townhalls` _outactors))
  (for _array_element _output_get
    (add `/Game/MyFirstRTS/Core/Building/BP_BuildingComponent.OnHealthZero` (`self.GetComponentByClass` _array_element "/Game/MyFirstRTS/Core/Building/BP_BuildingComponent.BP_BuildingComponent_C") (`|CreateDelegate` :!event `OnTownhallDestroyed`))))

(event `OnTownhallDestroyed`
  (params (BuildingRef :type "Actor Object Reference"))
  (`/Engine/EditorBlueprintResources/StandardMacros.IsValid` BuildingRef
    (:`Is Valid`
      (`KismetArrayLibrary.Array_RemoveItem` (`self.Townhalls`) BuildingRef)
      (if (`|EnumEquality` (`/Game/MyFirstRTS/Core/Building/BP_BuildingComponent.TeamAttitude` (`self.GetComponentByClass` BuildingRef "/Game/MyFirstRTS/Core/Building/BP_BuildingComponent.BP_BuildingComponent_C")) "Friendly")
        (`self.LoseTheGame`)))))

(event `LoseTheGame`
  (bind _returnvalue (`|CreateWidget` "/Game/MyFirstRTS/Core/UI/Screens/WBP_LoseScreen.WBP_LoseScreen_C"))
  (`UserWidget.AddToViewport` _returnvalue 0))

(fn `GetPlayerTownhall`
  (returns (TownHall :type "Actor Object Reference"))
  (locals (TownHallIndex :type Integer))
  (for _array_element (`self.Townhalls`)
    (bind _returnvalue (`KismetArrayLibrary.Array_Find` (`Actor.Tags` _array_element) "Player"))
    (if (>= _returnvalue 0)
      (set `local.TownHallIndex` _returnvalue)
      (break)))
  (return (`|GetArrayItem` (`self.Townhalls`) (`local.TownHallIndex`))))

(fn `UserConstructionScript`)