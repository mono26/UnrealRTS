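; BP_SelectionComponent is an RTS component that shows a selection indicator decal on its owning actor.
; On BeginPlay it adds a rotated decal using MI_SelectionIndicator, sizes and positions it from IndicatorRadius and IndicatorCenter, then hides it.
; OnSelected and OnDeselected toggle the decal's visibility and hidden-in-game state.
; CanBeSelected always returns true.
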(event `self.ReceiveBeginPlay`
  (bind _returnvalue (`|AddComponentByClass` (`self.GetOwner`) "/Script/Engine.DecalComponent" false (`KismetMathLibrary.MakeTransform` (0.0 0.0 0.0) (struct :`Pitch` 90.0))))
  (set `self.DecalComponentRef` _returnvalue)
  (`DecalComponent.SetDecalMaterial` (`self.DecalComponentRef`) "/Game/MyFirstRTS/Core/Building/MI_SelectionIndicator.MI_SelectionIndicator")
  (`self.UpdateDecal`)
  (`self.OnDeselected`))

(event `self.OnSelected`
  (bind _decalcomponentref (`self.DecalComponentRef`))
  (`SceneComponent.SetVisibility` _decalcomponentref true false)
  (`SceneComponent.SetHiddenInGame` _decalcomponentref false false))

(event `self.OnDeselected`
  (bind _decalcomponentref (`self.DecalComponentRef`))
  (`SceneComponent.SetVisibility` _decalcomponentref false false)
  (`SceneComponent.SetHiddenInGame` _decalcomponentref true false))

(fn `CanBeSelected`
  (returns (CanBeSelected :type Boolean))
  (return true))

(fn `UpdateDecal`
  (bind _decalcomponentref (`self.DecalComponentRef`))
  (bind _indicatorradius (`self.IndicatorRadius`))
  (bind (_decalsize_x _decalsize_y _decalsize_z) (`KismetMathLibrary.BreakVector` (`DecalComponent.DecalSize` (`self.DecalComponentRef`))))
  (`SceneComponent.SetRelativeScale3D` _decalcomponentref (`KismetMathLibrary.MakeVector` 128.0 (/ _indicatorradius _decalsize_y) (/ _indicatorradius _decalsize_z)))
  (`SceneComponent.K2_SetRelativeLocation` _decalcomponentref (`self.IndicatorCenter`) false false))