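; Actor component for health in an RTS, tracking damage on its owner and showing it through a health bar.
; On BeginPlay it adds a BP_HealthBarComponent to the owner at a configured offset and size, colored by the TeamComponent's attitude.
; It also binds to the owner's any-damage event, passing truncated damage to OnDamage and refreshing the bar with the current-to-max health ratio.
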(event `self.ReceiveBeginPlay`
  (bind _returnvalue (`self.GetOwner`))
  (`|ExecutionSequence`
    (:`then_0`
      (bind _returnvalue_2 (`|AddComponentByClass` _returnvalue "/Game/MyFirstRTS/Core/Unit/BP_HealthBarComponent.BP_HealthBarComponent_C" false (`KismetMathLibrary.MakeTransform` (`self.HealthBarLocalPos`))))
      (bind _output_get (set `self.HealthBarComponent` _returnvalue_2))
      (`WidgetComponent.SetDrawSize` _output_get (`self.HealthBarSize`))
      (`/Game/MyFirstRTS/Core/Unit/BP_HealthBarComponent.UpdateHealthBarColor` _output_get (select `ETeamAttitude` (`TeamComponent.TeamAttitude` (`Actor.GetComponentByClass` (`self.GetOwner`) "/Script/MyFirstRTS.TeamComponent")) :`Friendly` (struct :`G` 1.0 :`A` 1.0) :`Neutral` (struct :`R` 1.0 :`G` 1.0 :`A` 1.0) :`Hostile` (struct :`R` 1.0 :`A` 1.0) :!type "LinearColor Structure"))
      (`self.UpdateHealthBar`))
    (:`then_3`
      (add `Actor.OnTakeAnyDamage` _returnvalue (`|CreateDelegate` :!event `OnActorTakeAnyDamage`)))))

(event `self.UpdateHealthBar`
  (bind _returnvalue (`Actor.GetComponentByClass` (`self.GetOwner`) "/Game/MyFirstRTS/Core/Unit/BP_HealthBarComponent.BP_HealthBarComponent_C"))
  (`/Engine/EditorBlueprintResources/StandardMacros.IsValid` _returnvalue
    (:`Is Valid`
      (`/Game/MyFirstRTS/Core/Unit/BP_HealthBarComponent.UpdateHealthBar` _returnvalue (/ (`self.GetHealthCurrent`) (`self.GetMaxHealth`))))))

(event `OnActorTakeAnyDamage`
  (params (DamagedActor :type "Actor Object Reference") (Damage :type "Float (single-precision)") (DamageType :type "DamageType Object Reference") (InstigatedBy :type "Controller Object Reference") (DamageCauser :type "Actor Object Reference"))
  (`self.OnDamage` (`KismetMathLibrary.FTrunc` Damage))
  (`self.UpdateHealthBar`))