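; BP_EnemyCommander is the RTS enemy AI commander that starts spawning enemies shortly after play begins and sends them at the player's townhall.
; Each spawned enemy joins ActiveEnemies and receives an attack order through CommandComponent, with success and fail callbacks.
; The success handler reissues attacks on each unit's current UnitAttackComponent target, while the fail handler stops every active enemy.
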(event `self.ReceiveBeginPlay`
  (`KismetSystemLibrary.Delay` 2.0)
  (`self.StartSpawn`))

(event `self.OnSpawnEnemy`
  (params (Enemy :type "Actor Object Reference"))
  (`KismetArrayLibrary.Array_Add` (`self.ActiveEnemies`) Enemy)
  (bind _returnvalue (`self.GetPlayerTownhall`))
  (`CommanderComponent.ExecuteAttackCommand` (`self.CommandComponent`) _returnvalue Enemy (`|CreateDelegate` :!event `OnExecuteAttackSuccess`) (`|CreateDelegate` :!event `OnExecuteAttackFail`)))

(fn `OnExecuteAttackFail`
  (for _array_element (`self.ActiveEnemies`)
    (`CommanderComponent.ExecuteStopCommand` (`self.CommandComponent`) _array_element)))

(fn `OnExecuteAttackSuccess`
  (`KismetSystemLibrary.PrintString` "OnExecuteAttackSuccess")
  (for _array_element (`self.ActiveEnemies`)
    (bind _returnvalue (`Actor.GetComponentByClass` _array_element "/Script/MyFirstRTS.UnitAttackComponent"))
    (`/Engine/EditorBlueprintResources/StandardMacros.IsValid` _returnvalue
      (:`Is Valid`
        (`CommanderComponent.ExecuteAttackCommand` (`self.CommandComponent`) (`UnitAttackComponent.GetAttackTarget` _returnvalue) _array_element (`|CreateDelegate` :!event `OnExecuteAttackSuccess`) (`|CreateDelegate` :!event `OnExecuteAttackFail`))))))