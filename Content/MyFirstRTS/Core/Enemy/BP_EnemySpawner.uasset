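; Enemy spawner actor for an RTS that creates Tribe 2 worker units and reports spawn events to the enemy commander.
; GetSpawnPosition picks a random navigable point within its sphere's radius, raised slightly, and SpawnEnemy creates a worker at a given position.
; On BeginPlay it binds to the OnSpawnEnemy dispatcher, forwarding each enemy to BPEnemyCommander.
; Neither spawn function is called within this Blueprint.
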(event `self.ReceiveBeginPlay`
  (add `self.OnSpawnEnemy` (`|CreateDelegate` :!event `OnSpawnEnemyEvent`)))

(event `OnSpawnEnemyEvent` :!signature `self.OnSpawnEnemy`
  (params (Enemy :type "Actor Object Reference"))
  (`EnemyCommander.OnSpawnEnemy` (`self.BP_EnemyCommander`) Enemy))

(fn `GetSpawnPosition`
  (returns (ReturnValue :type "Vector Structure"))
  (bind _randomlocation (`NavigationSystemV1.K2_GetRandomLocationInNavigableRadius` (`self.K2_GetActorLocation`) (`SphereComponent.GetScaledSphereRadius` (`self.Sphere`)) null null))
  (return (+ _randomlocation (0.0 0.0 100.0))))

(fn `SpawnEnemy`
  (params (SpawnPosition :type "Vector Structure"))
  (returns (ReturnValue :type "Actor Object Reference"))
  (bind _returnvalue (`|SpawnActorFromClass` "/Game/MyFirstRTS/Units/Tribe2/BP_Worker_Tribe2.BP_Worker_Tribe2_C" (`KismetMathLibrary.MakeTransform` SpawnPosition) "Undefined" "OverrideRootScale" null null))
  (return _returnvalue))

(fn `UserConstructionScript`)