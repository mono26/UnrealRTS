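; AI controller for enemy units in an RTS that retargets a worker unit when its attack target is destroyed.
; OnTargetDestroyed clears the pawn's attack request, then asks the WorkerUnitBrainComponent for the next target in sight, falling back to the player townhall.
; Attack orders route through the owning commander's CommandComponent rather than being issued on the unit directly.
; BeginPlay, Tick and the construction script add no custom logic.
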(fn `OnTargetDestroyed`
  (bind _returnvalue (`self.GetComponentByClass` (`self.K2_GetPawn`) "/Script/MyFirstRTS.UnitAttackComponent"))
  (`KismetSystemLibrary.PrintString` "OnTargetDestroyed")
  (`/Engine/EditorBlueprintResources/StandardMacros.IsValid` _returnvalue
    (:`Is Valid`
      (`UnitAttackComponent.ClearAttackRequest` _returnvalue)
      (bind _returnvalue_2 (`WorkerUnitBrain.GetNextTargetInSight` (`self.WorkerUnitBrainComponent`)))
      (`/Engine/EditorBlueprintResources/StandardMacros.IsValid` _returnvalue_2
        (:`Is Valid`
          (bind _asbp_worker (cast `/Game/MyFirstRTS/Units/BP_Worker` (`self.K2_GetPawn`))
            (:`then`
              (`CommanderComponent.ExecuteAttackCommand` (`FactionCommander.CommandComponent` (`WorkerUnit.GetOwnerCommander` _asbp_worker)) _returnvalue_2 _asbp_worker (`|CreateDelegate` :!event `OnExecuteAttackSuccess`) (`|CreateDelegate` :!event `OnExecuteAttackFail`)))
            (:`CastFailed`
              (`KismetSystemLibrary.PrintString` "Not a valid worker." :!label _label))))
        (:`Is Not Valid`
          (bind _asbp_worker_2 (cast `/Game/MyFirstRTS/Units/BP_Worker` (`self.K2_GetPawn`))
            (:`then`
              (bind _returnvalue_3 (`WorkerUnit.GetOwnerCommander` _asbp_worker_2))
              (bind _returnvalue_4 (`FactionCommander.GetPlayerTownhall` _returnvalue_3))
              (`/Engine/EditorBlueprintResources/StandardMacros.IsValid` _returnvalue_4
                (:`Is Valid`
                  (`CommanderComponent.ExecuteAttackCommand` (`FactionCommander.CommandComponent` _returnvalue_3) _returnvalue_4 _asbp_worker_2 (`|CreateDelegate` :!event `OnExecuteAttackSuccess`) (`|CreateDelegate` :!event `OnExecuteAttackFail`)))))
            (:`CastFailed`
              (goto _label))))))
    (:`Is Not Valid`
      (goto _label))))

(fn `UserConstructionScript`
  (`parent.UserConstructionScript`))