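; Player controller for an RTS, handling camera panning, unit selection, orders and the player's resource stockpile.
; Keyboard axes move the controlled pawn, falling back to screen-edge mouse scrolling when idle.
; Selection input resizes a spawned BP_SelectionBox, while actor select, deselect and click events maintain SelectedActors.
; Action release sphere-overlaps the cursor hit to move workers or trigger interaction components, and received resources update the HUD.
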(event `self.ReceiveBeginPlay`
  (bind _returnvalue (`|SpawnActorFromClass` "/Game/MyFirstRTS/Core/Player/BP_SelectionBox.BP_SelectionBox_C" (`KismetMathLibrary.MakeTransform` (0.0 0.0 0.0)) "Undefined" "OverrideRootScale" null null))
  (set `self.SelectionBoxRef` _returnvalue))

(event `InputAxis|Movement_X_Keyboard`
  (params (AxisValue :type "Float (single-precision)"))
  (bind (_returnvalue_roll _returnvalue_pitch _returnvalue_yaw) (`KismetMathLibrary.BreakRotator` (`self.GetControlRotation`)))
  ;[1 1 1] Camera Horizontal Keyboard Input
  (`Pawn.AddMovementInput` (`self.K2_GetPawn`) (`KismetMathLibrary.GetForwardVector` (`KismetMathLibrary.MakeRotator` 0.0 0.0 _returnvalue_yaw)) (`KismetMathLibrary.SelectFloat` AxisValue (`self.MouseHorizontalScale`) (!= AxisValue 0.0)) false))

(event `InputAxis|Movement_Y_Keyboard`
  (params (AxisValue :type "Float (single-precision)"))
  (bind (_returnvalue_roll _returnvalue_pitch _returnvalue_yaw) (`KismetMathLibrary.BreakRotator` (`self.GetControlRotation`)))
  ;[1 1 1] Camera Vertical Keyboard Input
  (`Pawn.AddMovementInput` (`self.K2_GetPawn`) (* (`KismetMathLibrary.GetRightVector` (`KismetMathLibrary.MakeRotator` 0.0 0.0 _returnvalue_yaw)) (-1.0 -1.0 -1.0)) (`KismetMathLibrary.SelectFloat` AxisValue (`self.MouseVerticalScale`) (!= AxisValue 0.0)) false))

(event `InputAxis|Movement_Mouse`
  (params (AxisValue :type "Float (single-precision)"))
  (bind (_locationx _locationy) (`self.GetMousePosition`))
  (bind (_returnvalue_x _returnvalue_y) (`KismetMathLibrary.BreakVector2D` (`WidgetLayoutLibrary.GetViewportSize`)))
  (bind _viewportedgethreshold (`self.ViewportEdgeThreshold`))
  (bind _viewportedgethreshold_2 (`self.ViewportEdgeThreshold`))
  (bind _returnvalue (/ _locationx _returnvalue_x))
  (bind _returnvalue_2 (/ _locationy _returnvalue_y))
  ;[1 1 1] Camera Mouse Input
  (set `self.MouseHorizontalScale` (`KismetMathLibrary.SelectFloat` -1.0 (`KismetMathLibrary.SelectFloat` 1.0 0.0 (> _returnvalue (- 1.0 _viewportedgethreshold))) (< _returnvalue _viewportedgethreshold)))
  (set `self.MouseVerticalScale` (`KismetMathLibrary.SelectFloat` 1.0 (`KismetMathLibrary.SelectFloat` -1.0 0.0 (> _returnvalue_2 (- 1.0 _viewportedgethreshold_2))) (< _returnvalue_2 _viewportedgethreshold_2))))

(event `InputAction|Mouse_Selection`
  (params (Key :type "Key Structure"))
  (bind _selectionboxref (`self.SelectionBoxRef`))
  ;[1 1 1] Right Click
  (:`Pressed`
    (if (not (`self.IsClickSelecting`))
      (`self.DeselectActors`)
      (`self.K2_SetActorLocation` _selectionboxref (`.Location` (`GameplayStatics.BreakHitResult` (`self.GetHitResultUnderCursorByChannel` "TraceTypeQuery1"))) false false)
      (`/Game/MyFirstRTS/Core/Player/BP_SelectionBox.ActivateResizing` _selectionboxref true)
      (`/Game/MyFirstRTS/Core/Player/BP_SelectionBox.ActivateResizing` _selectionboxref true)))
  (:`Released`
    (if (not (`self.IsClickSelecting`))
      (`/Game/MyFirstRTS/Core/Player/BP_SelectionBox.ActivateResizing` _selectionboxref false)
      (else
        (set `self.IsClickSelecting` false)))))

(event `InputAction|Mouse_Action`
  (params (Key :type "Key Structure"))
  ;[1 1 1] Left Click
  (:`Released`
    (if (`KismetArrayLibrary.Array_IsNotEmpty` (`self.SelectedActors`))
      (bind _outactors (`KismetSystemLibrary.SphereOverlapActors` (`.Location` (`GameplayStatics.BreakHitResult` (`self.GetHitResultUnderCursorByChannel` "TraceTypeQuery1"))) 50.0 (`|MakeArray` "ObjectTypeQuery2" "ObjectTypeQuery3" :!type "EObjectTypeQuery Enum")))
      (if (`KismetArrayLibrary.Array_IsEmpty` _outactors)
        (`self.MoveSelection`)
        (else
          (for _array_element (`self.SelectedActors`)
            (bind _output (`|GetArrayItem` _outactors))
            (`/Engine/EditorBlueprintResources/StandardMacros.IsValid` (`self.GetComponentByClass` _output "/Game/MyFirstRTS/Core/Building/BP_InteractableComponent.BP_InteractableComponent_C")
              (:`Is Valid`
                (bind _returnvalue (`self.GetComponentByClass` _array_element "/Game/MyFirstRTS/Core/Unit/BP_InteractionComponent.BP_InteractionComponent_C"))
                (`/Engine/EditorBlueprintResources/StandardMacros.IsValid` _returnvalue
                  (:`Is Valid`
                    (`/Game/MyFirstRTS/Core/Unit/BP_InteractionComponent.InteractWith` _returnvalue _output)
                    (`NiagaraFunctionLibrary.SpawnSystemAtLocation` "/Game/MyFirstRTS/Core/Player/NS_ClickIndicator.NS_ClickIndicator" (`self.K2_GetActorLocation` _output) (struct) (1.0 1.0 1.0) true true "AutoRelease"))))
              (:`Is Not Valid`
                (`KismetSystemLibrary.PrintString` "No interactable component found")))))))))

(event `OnActorSelected`
  (params (SelectedActor :type "Actor Object Reference"))
  (`KismetArrayLibrary.Array_Add` (`self.SelectedActors`) SelectedActor))

(event `OnGameActorClicked`
  (params (ClickedActor :type "Actor Object Reference"))
  (set `self.IsClickSelecting` true)
  (`self.DeselectActors`)
  (message `/Game/MyFirstRTS/Core/Building/BPI_ISelectable.OnSelected` ClickedActor))

(event `OnActorDeselected`
  (params (DeselectedActor :type "Actor Object Reference"))
  (`KismetArrayLibrary.Array_RemoveItem` (`self.SelectedActors`) DeselectedActor))

(fn `DeselectActors`
  (bind _selectedactors (`self.SelectedActors`))
  (for _array_element _selectedactors
    (if (`KismetSystemLibrary.DoesImplementInterface` _array_element "/Game/MyFirstRTS/Core/Building/BPI_ISelectable.BPI_ISelectable_C")
      (message `/Game/MyFirstRTS/Core/Building/BPI_ISelectable.OnDeselected` _array_element)))
  (`KismetArrayLibrary.Array_Clear` _selectedactors))

(fn `MoveSelection`
  (for _array_element (`self.SelectedActors`)
    (bind _asbp_worker (cast `/Game/MyFirstRTS/Units/BP_Worker` _array_element))
    (`WorkerUnit.ExecuteCommand` _asbp_worker null)
    (`NiagaraFunctionLibrary.SpawnSystemAtLocation` "/Game/MyFirstRTS/Core/Player/NS_ClickIndicator.NS_ClickIndicator" (0.0 0.0 0.0) (struct) (1.0 1.0 1.0) true true "AutoRelease")))

(fn `ReceiveResources`
  (params (ResourceType :type "/Game/MyFirstRTS/Core/Resource/E_ResourceType Enum" :default "NewEnumerator0") (ResourceAmount :type Integer))
  (bind _storedresources (`self.StoredResources`))
  (bind _resourcetype (`local.ResourceType`))
  (bind _storedresources_2 (`self.StoredResources`))
  (bind _resourcetype_2 (`local.ResourceType`))
  (`|ExecutionSequence`
    (:`then_0`
      (if (`BlueprintMapLibrary.Map_Contains` _storedresources ResourceType)
        (`BlueprintMapLibrary.Map_Add` _storedresources_2 _resourcetype_2 (+ (`BlueprintMapLibrary.Map_Find` _storedresources_2 _resourcetype_2) (`local.ResourceAmount`)))
        (else
          (`BlueprintMapLibrary.Map_Add` _storedresources (`local.ResourceType`) (`local.ResourceAmount`)))))
    (:`then_1`
      (bind _asbp_hud (cast `/Game/MyFirstRTS/Core/UI/HUD/BP_HUD` (`self.GetHUD`)))
      (`/Game/MyFirstRTS/Core/UI/HUD/WBP_HUD.UpdateResourceValue` (`/Game/MyFirstRTS/Core/UI/HUD/BP_HUD.WidgetRef` _asbp_hud) _resourcetype (`BlueprintMapLibrary.Map_Find` (`self.StoredResources`) _resourcetype)))))

(fn `UserConstructionScript`)