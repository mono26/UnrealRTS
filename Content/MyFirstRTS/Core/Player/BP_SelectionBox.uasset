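; BP_SelectionBox is the RTS drag-selection actor that selects units inside a world-space box.
; While resizing, Tick stretches BoxArea between the actor's origin and the cursor's visibility-trace hit, then updates the HUD widget's selection box.
; Overlaps message BPI_ISelectable actors that can be selected: entering selects, leaving deselects only while resizing.
; ActivateResizing toggles box collision and the HUD box, so units stay selected when collision switches off.
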(event `self.ReceiveTick`
  (params (DeltaSeconds :type "Float (single-precision)"))
  (bind _boxarea (`self.BoxArea`))
  (bind (_returnvalue_x _returnvalue_y) (`KismetMathLibrary.BreakVector` (/ (`KismetMathLibrary.Vector_GetAbs` (- (`self.K2_GetActorLocation`) (`self.CursorPosition`))) 2.0)))
  ;[1 1 1] Resize Box
  (if (`self.ShouldResize`)
    (bind _aspc_my_first_rts (cast `/Game/MyFirstRTS/Core/Player/BP_PlayerCommander` (`GameplayStatics.GetPlayerController` 0)))
    (bind _output_get (set `self.CursorPosition` (`.Location` (`GameplayStatics.BreakHitResult` (`PlayerController.GetHitResultUnderCursorByChannel` _aspc_my_first_rts "TraceTypeQuery1" true)))))
    (bind (_x _y) (`KismetMathLibrary.BreakVector3f` (`KismetMathLibrary.VLerp` (`self.K2_GetActorLocation`) _output_get 0.5)))
    (`SceneComponent.K2_SetWorldLocation` _boxarea (`KismetMathLibrary.MakeVector` _x _y 150.0) false false)
    (`BoxComponent.SetBoxExtent` _boxarea (`KismetMathLibrary.MakeVector` _returnvalue_x _returnvalue_y 300.0) true)
    (bind _asbp_hud (cast `/Game/MyFirstRTS/Core/UI/HUD/BP_HUD` (`PlayerController.GetHUD` (`GameplayStatics.GetPlayerController` 0))))
    (`/Game/MyFirstRTS/Core/UI/HUD/WBP_HUD.UpdateSelectionBox` (`/Game/MyFirstRTS/Core/UI/HUD/BP_HUD.WidgetRef` _asbp_hud))))

(event `self.BoxArea.OnComponentBeginOverlap`
  (params (OverlappedComponent :type "PrimitiveComponent Object Reference") (OtherActor :type "Actor Object Reference") (OtherComp :type "PrimitiveComponent Object Reference") (OtherBodyIndex :type Integer) (bFromSweep :type Boolean) (SweepResult :type "HitResult Structure (by ref)"))
  (if (`KismetSystemLibrary.DoesImplementInterface` OtherActor "/Game/MyFirstRTS/Core/Building/BPI_ISelectable.BPI_ISelectable_C")
    (bind _canbeselected (message `/Game/MyFirstRTS/Core/Building/BPI_ISelectable.CanBeSelected` OtherActor))
    (if _canbeselected
      (message `/Game/MyFirstRTS/Core/Building/BPI_ISelectable.OnSelected` OtherActor))))

(event `self.BoxArea.OnComponentEndOverlap`
  (params (OverlappedComponent :type "PrimitiveComponent Object Reference") (OtherActor :type "Actor Object Reference") (OtherComp :type "PrimitiveComponent Object Reference") (OtherBodyIndex :type Integer))
  (if (and (`self.ShouldResize`) (`KismetSystemLibrary.DoesImplementInterface` OtherActor "/Game/MyFirstRTS/Core/Building/BPI_ISelectable.BPI_ISelectable_C"))
    (bind _canbeselected (message `/Game/MyFirstRTS/Core/Building/BPI_ISelectable.CanBeSelected` OtherActor))
    (if _canbeselected
      (message `/Game/MyFirstRTS/Core/Building/BPI_ISelectable.OnDeselected` OtherActor))))

(fn `ActivateResizing`
  (params (Resize :type Boolean))
  (bind _boxarea (`self.BoxArea`))
  (bind _returnvalue (`PlayerController.GetHUD` (`GameplayStatics.GetPlayerController` 0)))
  (bind _output_get (set `self.ShouldResize` Resize))
  (if _output_get
    (`PrimitiveComponent.SetCollisionEnabled` _boxarea "QueryOnly")
    (bind _asbp_hud (cast `/Game/MyFirstRTS/Core/UI/HUD/BP_HUD` _returnvalue))
    (`/Game/MyFirstRTS/Core/UI/HUD/WBP_HUD.ActivateSelectionBox` (`/Game/MyFirstRTS/Core/UI/HUD/BP_HUD.WidgetRef` _asbp_hud) true)
    (else
      (`PrimitiveComponent.SetCollisionEnabled` _boxarea "NoCollision")
      (bind _asbp_hud_2 (cast `/Game/MyFirstRTS/Core/UI/HUD/BP_HUD` _returnvalue))
      (`/Game/MyFirstRTS/Core/UI/HUD/WBP_HUD.ActivateSelectionBox` (`/Game/MyFirstRTS/Core/UI/HUD/BP_HUD.WidgetRef` _asbp_hud_2) false))))

(fn `UserConstructionScript`)