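; BP_Worker is an RTS worker unit that forwards click and selection to BPUnitComponent, plays state-based animations and destroys itself after health reaches zero.
; ExecuteAttack uses AIMoveTo to reach the target's closest InteractableComponent point, retrying on failure, then records range and starts a looping timer.
; DealAttackDamage applies damage within that range, otherwise stops the timer and re-attacks if still Attacking.
; SetTarget is empty; its team-check logic is disconnected.
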(event `self.ReceiveBeginPlay`)

(event `self.ReceiveActorOnClicked`
  (params (ButtonPressed :type "Key Structure"))
  ;[1 1 1] IClickable
  (`self.OnCursorClicked`))

(event `self.OnCursorClicked`
  ;[1 1 1] IClickable
  (`/Game/MyFirstRTS/Core/Unit/BP_UnitComponent.OnCursorClicked` (`self.BP_UnitComponent`)))

(event `/Game/MyFirstRTS/Core/Building/BPI_ISelectable.OnSelected`
  ;[1 1 1] ISelectable
  (`/Game/MyFirstRTS/Core/Unit/BP_UnitComponent.OnSelected` (`self.BP_UnitComponent`)))

(event `/Game/MyFirstRTS/Core/Building/BPI_ISelectable.OnDeselected`
  ;[1 1 1] ISelectable
  (`/Game/MyFirstRTS/Core/Unit/BP_UnitComponent.OnDeselected` (`self.BP_UnitComponent`)))

(event `self.OnStartMovement`
  (`KismetSystemLibrary.K2_ClearAndInvalidateTimerHandle` (`self.AttackTimer`)))

(event `self.BP_UnitComponent.OnCurrentStateChanged`
  (bind _returnvalue (`UnitComponent.GetCurrentState` (`self.BP_UnitComponent`)))
  (`SkeletalMeshComponent.PlayAnimation` (`self.Mesh`) (select `EUnitStates` _returnvalue :`Idle` "/Game/StrategyGameAssets/Characters/DwarfGrunt/Anims/Idle_1_new.Idle_1_new" :`Moving` "/Game/StrategyGameAssets/Characters/DwarfGrunt/Anims/WalkFwd2.WalkFwd2" :`Gathering` "/Game/StrategyGameAssets/Characters/DwarfGrunt/Anims/AnimMontageAttack_1_new.AnimMontageAttack_1_new" :`Attacking` "/Game/StrategyGameAssets/Characters/DwarfGrunt/Anims/AnimMontageAttack_1_new.AnimMontageAttack_1_new" :!type "AnimationAsset Object Reference") true))

(event `self.CapsuleComponent.OnClicked`
  (params (TouchedComponent :type "PrimitiveComponent Object Reference") (ButtonPressed :type "Key Structure"))
  (`self.OnCursorClicked`))

(event `self.ExecuteAttack`
  (bind _returnvalue (`self.K2_GetActorLocation`))
  (bind _bp_unitcomponent (`self.BP_UnitComponent`))
  ;[1 1 1] IAttacker
  (`KismetSystemLibrary.K2_ClearAndInvalidateTimerHandle` (`self.AttackTimer`))
  (bind _returnvalue_2 (`self.GetAttackTarget`))
  (`/Engine/EditorBlueprintResources/StandardMacros.IsValid` _returnvalue_2
    (:`Is Valid`
      (`UnitComponent.SetCurrentState` _bp_unitcomponent "Moving")
      (bind _returnvalue_3 (`self.GetComponentByClass` _returnvalue_2 "/Script/MyFirstRTS.InteractableComponent"))
      (`/Engine/EditorBlueprintResources/StandardMacros.IsValid` _returnvalue_3
        (:`Is Valid`
          (`InteractableComponent.GetInteractableRadius` _returnvalue_3)
          (`UnitComponent.SetCurrentState` _bp_unitcomponent "Moving")
          (bind _returnvalue_4 (`InteractableComponent.GetClosestInteractionPointTo` _returnvalue_3 self))
          (`/Engine/EditorBlueprintResources/StandardMacros.IsValid` _returnvalue_4
            (:`Is Valid`
              (`|AIMoveTo` self (+ (`SceneComponent.K2_GetComponentLocation` _returnvalue_4) (0.0 0.0 0.1)) null 50.0
                (:`OnSuccess`
                  (bind _returnvalue_5 (`self.GetAttackTarget` :!label _label))
                  (`/Engine/EditorBlueprintResources/StandardMacros.IsValid` _returnvalue_5
                    (:`Is Valid`
                      (bind _returnvalue_6 (`self.K2_GetActorLocation` _returnvalue_5))
                      (set `self.RangeToTarget` (`KismetMathLibrary.Vector_Distance` _returnvalue _returnvalue_6))
                      (bind (_returnvalue_roll _returnvalue_pitch _returnvalue_yaw) (`KismetMathLibrary.BreakRotator` (`KismetMathLibrary.FindLookAtRotation` _returnvalue _returnvalue_6)))
                      (`self.K2_SetActorRotation` (`KismetMathLibrary.MakeRotator` 0.0 0.0 _returnvalue_yaw))
                      (`UnitComponent.SetCurrentState` (`self.BP_UnitComponent`) "None")
                      (bind _returnvalue_7 (`KismetSystemLibrary.K2_SetTimerDelegate` (`|CreateDelegate` :!event `DealAttackDamage`) 1.0 true))
                      (set `self.AttackTimer` _returnvalue_7))
                    (:`Is Not Valid`
                      (`UnitComponent.SetCurrentState` (`self.BP_UnitComponent`) "Idle"))))
                (:`OnFail`
                  (`self.ExecuteAttack` :!label _label_2))))
            (:`Is Not Valid`
              (bind _returnvalue_8 (`self.GetAttackTarget`))
              (`|AIMoveTo` self (0.0 0.0 0.0) _returnvalue_8 50.0
                (:`OnSuccess`
                  (goto _label))
                (:`OnFail`
                  (goto _label_2))))))
        (:`Is Not Valid`
          (`KismetSystemLibrary.PrintString` "Can't attack target"))))
    (:`Is Not Valid`
      (`KismetSystemLibrary.PrintString` "No target to attack." true true (struct :`G` 0.66 :`B` 1.0 :`A` 1.0) 10.0))))

(event `self.DealAttackDamage`
  ;[1 1 1] IAttacker
  (bind _returnvalue (`self.GetAttackTarget`))
  (`/Engine/EditorBlueprintResources/StandardMacros.IsValid` _returnvalue
    (:`Is Valid`
      (bind _returnvalue_2 (`self.GetAttackTarget`))
      (if (<= (`KismetMathLibrary.Vector_Distance` (`self.K2_GetActorLocation`) (`self.K2_GetActorLocation` _returnvalue_2)) (`self.RangeToTarget`))
        (bind _returnvalue_3 (`self.GetAttackTarget`))
        (`GameplayStatics.ApplyDamage` _returnvalue_3 (`UnitComponent.AttackDamage` (`self.BP_UnitComponent`)) null self)
        (else
          (`KismetSystemLibrary.K2_ClearAndInvalidateTimerHandle` (`self.AttackTimer`))
          (bind _returnvalue_4 (`UnitComponent.GetCurrentState` (`self.BP_UnitComponent`)))
          (if (`|EnumEquality` _returnvalue_4 "Attacking")
            (`self.ExecuteAttack`)))))
    (:`Is Not Valid`
      (`UnitComponent.SetCurrentState` (`self.BP_UnitComponent`) "Idle")
      (`KismetSystemLibrary.K2_ClearAndInvalidateTimerHandle` (`self.AttackTimer`)))))

(event `self.BP_UnitComponent.OnHealthZero`
  (params (UnitRef :type "Actor Object Reference"))
  (bind _capsulecomponent (`self.CapsuleComponent`))
  (`SceneComponent.SetVisibility` _capsulecomponent false false)
  (`SceneComponent.SetHiddenInGame` _capsulecomponent false false)
  (`KismetSystemLibrary.Delay` 0.5)
  (`self.K2_DestroyActor`))

(event `self.SetTarget`
  (params (TargetRef :type "Actor Object Reference")))

(event `self.OnStopAll`
  (`KismetSystemLibrary.K2_ClearAndInvalidateTimerHandle` (`self.AttackTimer`)))

(fn `CanBeSelected`
  (returns (CanBeSelected :type Boolean))
  (bind _canbeselected (`/Game/MyFirstRTS/Core/Unit/BP_UnitComponent.CanBeSelected` (`self.BP_UnitComponent`)))
  (return _canbeselected))

(fn `UserConstructionScript`)