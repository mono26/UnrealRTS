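; RTS unit Blueprint with click and selection interface hooks, state-driven animation and death handling.
; Unit component state changes play looping mesh animations directly, with gathering and attacking sharing one attack montage.
; Actor and capsule clicks route to OnCursorClicked, while CanBeSelected returns false here and the stop-all event is empty.
; When the health component reaches zero, it turns off capsule visibility and destroys the actor after a short delay.
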(event `self.ReceiveActorOnClicked`
  (params (ButtonPressed :type "Key Structure"))
  ;[1 1 1] IClickable
  (`self.OnCursorClicked`))

(event `self.OnCursorClicked`
  ;[1 1 1] IClickable
  (`/Game/MyFirstRTS/Core/Unit/BP_UnitComponent.OnCursorClicked`))

(event `/Game/MyFirstRTS/Core/Component/BPI_ISelectable.OnSelected`
  ;[1 1 1] ISelectable
  (`/Game/MyFirstRTS/Core/Unit/BP_UnitComponent.OnSelected`))

(event `/Game/MyFirstRTS/Core/Component/BPI_ISelectable.OnDeselected`
  ;[1 1 1] ISelectable
  (`/Game/MyFirstRTS/Core/Unit/BP_UnitComponent.OnDeselected`))

(event `CustomEvent`)

(event `self.OnStopAll`)

(event `self.BP_UnitComponent.OnCurrentStateChanged`
  (bind _returnvalue (`UnitComponent.GetCurrentState` (`self.BP_UnitComponent`)))
  (`SkeletalMeshComponent.PlayAnimation` (`self.Mesh`) (select `EUnitStates` _returnvalue :`Idle` "/Game/StrategyGameAssets/Characters/DwarfGrunt/Anims/Idle_1_new.Idle_1_new" :`Moving` "/Game/StrategyGameAssets/Characters/DwarfGrunt/Anims/WalkFwd2.WalkFwd2" :`Gathering` "/Game/StrategyGameAssets/Characters/DwarfGrunt/Anims/AnimMontageAttack_1_new.AnimMontageAttack_1_new" :`Attacking` "/Game/StrategyGameAssets/Characters/DwarfGrunt/Anims/AnimMontageAttack_1_new.AnimMontageAttack_1_new" :!type "AnimationAsset Object Reference") true))

(event `self.CapsuleComponent.OnClicked`
  (params (TouchedComponent :type "PrimitiveComponent Object Reference") (ButtonPressed :type "Key Structure"))
  (`self.OnCursorClicked`))

(event `self.BP_HealthComponent.OnHealthZero`
  (bind _capsulecomponent (`self.CapsuleComponent`))
  (`SceneComponent.SetVisibility` _capsulecomponent false false)
  (`SceneComponent.SetHiddenInGame` _capsulecomponent false false)
  (`KismetSystemLibrary.Delay` 0.5)
  (`self.K2_DestroyActor`))

(fn `CanBeSelected`
  (returns (CanBeSelected :type Boolean))
  (return false))

(fn `UserConstructionScript`)